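; BP_Prefab_RuinPillar is a ruin pillar prefab that picks a random static mesh for itself when play begins.
; BeginPlay sets the StaticMesh component from the Allowedmeshes array, then calls the parent BeginPlay.
; The random index has one subtracted, so it can be -1 and never selects the last entry.
; The construction script only calls its parent, so the random choice happens only at runtime.
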(event `self.ReceiveBeginPlay`
  (`StaticMeshComponent.SetStaticMesh` (`self.StaticMesh`) (`KismetArrayLibrary.Array_Get` (`self.Allowedmeshes`) (- (`KismetMathLibrary.RandomInteger` (`KismetArrayLibrary.Array_Length` (`self.Allowedmeshes`))) 1)))
  (`parent.ReceiveBeginPlay`))

(fn `UserConstructionScript`
  (`parent.UserConstructionScript`))